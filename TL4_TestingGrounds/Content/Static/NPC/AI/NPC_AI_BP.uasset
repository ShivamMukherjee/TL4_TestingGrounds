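; AI controller for guard NPCs that runs the GuardBehaviour tree on the PatrolData blackboard.
; AI perception updates write a sensed actor to the blackboard's enemy key and clear that key when a stimulus is not successfully sensed.
; Actors carrying the controlled pawn's first tag are ignored, so that tag acts as a simple team filter.
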(event `self.ReceiveBeginPlay`
  (bind _blackboardcomponent (`self.UseBlackboard` "/Game/Static/NPC/AI/PatrolData.PatrolData"))
  (`self.RunBehaviorTree` "/Game/Static/NPC/AI/GuardBehaviour.GuardBehaviour"))

(event `self.AIPerception.OnTargetPerceptionUpdated`
  (params (Actor :type "Actor Object Reference") (Stimulus :type "AIStimulus Structure"))
  (bind _enemykey (`self.EnemyKey`))
  (if (`self.ActorHasTag` Actor (`|GetArrayItem` (`Actor.Tags` (`self.K2_GetPawn`))))
    _
    (elif (`.bSuccessfullySensed` (break `AIStimulus` Stimulus))
      (`BlackboardComponent.SetValueAsObject` (stale `self.ReceiveBeginPlay` _blackboardcomponent) _enemykey Actor)
      (else
        (`BlackboardComponent.ClearValue` (stale `self.ReceiveBeginPlay` _blackboardcomponent) _enemykey)))))

(fn `UserConstructionScript`)
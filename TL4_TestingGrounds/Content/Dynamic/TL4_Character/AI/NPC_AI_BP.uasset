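; AI controller for NPC-controlled TL4_Character pawns, running guard behavior with enemy detection.
; On BeginPlay it sets up the PatrolData blackboard and runs the GuardBehaviour tree.
; AI Perception writes sensed actors lacking the pawn's first tag to EnemyKey, treating that tag as a team marker, and clears the key on lost sight or other failed sensing.
; Tick sets the character's Aiming and Shooting flags whenever a focus actor is valid.
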(event `self.ReceiveTick`
  (params (DeltaSeconds :type "Float (single-precision)"))
  (bind _returnvalue (`KismetSystemLibrary.IsValid` (`self.GetFocusActor`)))
  (bind _astl4_character (cast `/Game/Dynamic/TL4_Character/Behaviour/TL4_Character` (`self.K2_GetPawn`)))
  (set `/Game/Dynamic/TL4_Character/Behaviour/TL4_Character.Aiming` _returnvalue _astl4_character)
  (set `/Game/Dynamic/TL4_Character/Behaviour/TL4_Character.Shooting` _returnvalue _astl4_character))

(event `self.ReceiveBeginPlay`
  (bind _blackboardcomponent (`self.UseBlackboard` "/Game/Dynamic/TL4_Character/AI/PatrolData.PatrolData"))
  (`self.RunBehaviorTree` "/Game/Dynamic/TL4_Character/AI/GuardBehaviour.GuardBehaviour"))

(event `self.AIPerception.OnTargetPerceptionUpdated`
  (params (Actor :type "Actor Object Reference") (Stimulus :type "AIStimulus Structure"))
  (bind _enemykey (`self.EnemyKey`))
  (if (`self.ActorHasTag` Actor (`|GetArrayItem` (`Actor.Tags` (`self.K2_GetPawn`))))
    _
    (elif (`.bSuccessfullySensed` (break `AIStimulus` Stimulus))
      (`BlackboardComponent.SetValueAsObject` (stale `self.ReceiveBeginPlay` _blackboardcomponent) _enemykey Actor)
      (else
        (`BlackboardComponent.ClearValue` (stale `self.ReceiveBeginPlay` _blackboardcomponent) _enemykey)))))

(fn `UserConstructionScript`)
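; AI controller for guard NPCs that runs the guard behavior tree on a patrol blackboard from BeginPlay.
; AI perception updates feed the blackboard's enemy key, treating any actor that lacks the controlled pawn's first tag as an enemy.
; A successful sense stores that actor, and a failed one clears the key without checking which actor it holds.
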(event `self.ReceiveBeginPlay`
  (bind _blackboardcomponent (`self.UseBlackboard` "/Game/Dynamic/TL4Character/AI/BB_PatrolData.BB_PatrolData"))
  (set `self.Blackboard Component` _blackboardcomponent)
  (`self.RunBehaviorTree` "/Game/Dynamic/TL4Character/AI/BT_GuardBehaviour.BT_GuardBehaviour"))

(event `self.AIPerception.OnTargetPerceptionUpdated`
  (params (Actor :type "Actor Object Reference") (Stimulus :type "AIStimulus Structure"))
  (`self.Update Blackboard Enemy Key` Actor Stimulus Actor))

(fn `Update Blackboard Enemy Key`
  (params (ControlledActor :type "Actor Object Reference") (AIStimulus :type "AIStimulus Structure (by ref)") (ObjectValue :type "Actor Object Reference"))
  (bind _blackboard_component (`self.Blackboard Component`))
  (bind _enemykey (`self.EnemyKey`))
  (`/Engine/EditorBlueprintResources/StandardMacros.IsValid` ControlledActor
    (:`Is Valid`
      (if (`self.ActorHasTag` ControlledActor (`|GetArrayItem` (`Actor.Tags` (`self.K2_GetPawn`))))
        _
        (elif (`.bSuccessfullySensed` (break `AIStimulus` AIStimulus))
          (`BlackboardComponent.SetValueAsObject` _blackboard_component _enemykey ObjectValue)
          (else
            (`BlackboardComponent.ClearValue` _blackboard_component _enemykey)))))))

(fn `UserConstructionScript`)